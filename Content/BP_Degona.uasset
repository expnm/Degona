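; BP_Degona is a character Blueprint that lets the player adjust the sock length on its skeletal mesh and switch camera views.
; Up and down inputs step a clamped SocksLength value and write it to the mesh materials as a scalar parameter, which is also applied on BeginPlay.
; A camera input uses a FlipFlop to alternate between body and face cameras by activating one and deactivating the other.
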(event `self.ReceiveBeginPlay`
  (`MeshComponent.SetScalarParameterValueOnMaterials` (`self.SkeletalMesh`) "SocksLength" (`self.SocksLength`)))

(event `InputAction|ChangeSocksLengthUp`
  (params (Key :type "Key Structure"))
  ;[1 1 1] change socks length
  (:`Pressed`
    (set `self.SocksLength` (`KismetMathLibrary.FClamp` (+ (`self.SocksLength`) (`self.SocksLengthStep`))))
    (`MeshComponent.SetScalarParameterValueOnMaterials` (`self.SkeletalMesh`) "SocksLength" (`self.SocksLength`) :!label _label)))

(event `InputAction|ChangeSocksLengthDown`
  (params (Key :type "Key Structure"))
  ;[1 1 1] change socks length
  (:`Pressed`
    (set `self.SocksLength` (`KismetMathLibrary.FClamp` (- (`self.SocksLength`) (`self.SocksLengthStep`))))
    (goto _label)))

(event `InputAction|ChangeCamera`
  (params (Key :type "Key Structure"))
  ;[1 1 1] change camera
  (:`Pressed`
    (`/Engine/EditorBlueprintResources/StandardMacros.FlipFlop`
      (:`A`
        (`ActorComponent.Deactivate` (`self.CameraBody`))
        (`ActorComponent.Activate` (`self.CameraFace`) false))
      (:`B`
        (`ActorComponent.Deactivate` (`self.CameraFace`))
        (`ActorComponent.Activate` (`self.CameraBody`) false)))))

(fn `UserConstructionScript`)